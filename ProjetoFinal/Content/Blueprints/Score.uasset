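; Score display actor that shows an integer counter, Placar, in the world through a TextRender component.
; BeginPlay writes the initial value padded to at least four digits without grouping.
; The AdicionaPlacar event adds one point and refreshes the text, but does not pass the same padding options.
; Tick, overlap and construction logic are empty.
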(event `AdicionaPlacar`
  (bind _output_get (set `self.Placar` (+ (`self.Placar`) 1)))
  (`TextRenderComponent.K2_SetText` (`self.TextRender`) (`KismetTextLibrary.Conv_IntToText` _output_get false false 4)))

(event `self.ReceiveBeginPlay`
  (`TextRenderComponent.K2_SetText` (`self.TextRender`) (`KismetTextLibrary.Conv_IntToText` (`self.Placar`) false false 4)))

(fn `UserConstructionScript`)