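; Launcher actor that repeatedly spawns Fruta (fruit) actors at its Arrow component and flings them with a radial impulse.
; StartGame1 waits a random delay, then loops through spawn, mass-independent impulse on the fruit's ProceduralMesh and another random delay, with no stop condition.
; A similar loop for FrutaEspecial, with longer delays and a weaker impulse, is disconnected and never runs.
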(event `self.ReceiveBeginPlay`)

(event `StartGame1`
  (bind (_returnvalue_location _returnvalue_rotation) (`KismetMathLibrary.BreakTransform` (`SceneComponent.K2_GetComponentToWorld` (`self.Arrow`))))
  (`KismetSystemLibrary.Delay` (`KismetMathLibrary.RandomFloatInRange` 0.0 2.0))
  (bind _returnvalue (`|SpawnActorFromClass` "/Game/Blueprints/Fruta.Fruta_C" (`KismetMathLibrary.MakeTransform` _returnvalue_location _returnvalue_rotation) "Undefined" "MultiplyWithRoot" null null :!label _label))
  (bind _proceduralmesh (`/Game/Blueprints/Fruta.ProceduralMesh` _returnvalue))
  (`PrimitiveComponent.AddRadialImpulse` _proceduralmesh (`SceneComponent.K2_GetComponentLocation` _proceduralmesh) 50.0 825.0 "RIF_Constant" true)
  (`KismetSystemLibrary.Delay` (`KismetMathLibrary.RandomFloatInRange` 0.5 2.5))
  (goto _label))

(fn `UserConstructionScript`)