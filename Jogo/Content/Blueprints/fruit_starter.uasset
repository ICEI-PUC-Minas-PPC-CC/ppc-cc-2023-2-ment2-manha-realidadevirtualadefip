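; Start-trigger fruit that begins the game when a Katana touches it.
; Construction copies a static mesh into a procedural mesh with collision, which BeginPlay spins continuously through a looping MoveComponentTo and short delay.
; When the Katana overlaps its sphere, the mesh gets gravity enabled and the Launcher and Launcher2 actors are found by class and told to start their games.
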(event `self.ReceiveBeginPlay`
  (bind _proceduralmesh (`self.ProceduralMesh`))
  (bind (_relativerotation_roll _relativerotation_pitch _relativerotation_yaw) (`KismetMathLibrary.BreakRotator` (`SceneComponent.RelativeRotation` _proceduralmesh)))
  (`KismetSystemLibrary.MoveComponentTo` _proceduralmesh (`SceneComponent.RelativeLocation` _proceduralmesh) (`KismetMathLibrary.MakeRotator` _relativerotation_roll _relativerotation_pitch (+ _relativerotation_yaw 180.0)) false false 2.0 :!label _label)
  (`KismetSystemLibrary.Delay` 0.01)
  (goto _label))

(event `self.Sphere.OnComponentBeginOverlap`
  (params (OverlappedComponent :type "PrimitiveComponent Object Reference") (OtherActor :type "Actor Object Reference") (OtherComp :type "PrimitiveComponent Object Reference") (OtherBodyIndex :type Integer) (bFromSweep :type Boolean) (SweepResult :type "HitResult Structure (by ref)"))
  (cast `/Game/Blueprints/Katana` OtherActor)
  (`PrimitiveComponent.SetEnableGravity` (`self.ProceduralMesh`) true)
  (bind _returnvalue (`GameplayStatics.GetActorOfClass` "/Game/Blueprints/launcher.launcher_C"))
  (`/Game/Blueprints/launcher.StartGame` _returnvalue)
  (bind _returnvalue_2 (`GameplayStatics.GetActorOfClass` "/Game/Blueprints/launcher2.launcher2_C"))
  (`/Game/Blueprints/launcher2.StartGame2` _returnvalue_2))

(fn `UserConstructionScript`
  (`KismetProceduralMeshLibrary.CopyProceduralMeshFromStaticMeshComponent` (`self.HierarchicalInstancedStaticMesh`) 0 (`self.ProceduralMesh`) true))